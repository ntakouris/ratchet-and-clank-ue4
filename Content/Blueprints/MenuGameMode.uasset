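; MenuGameMode is the game mode for the main menu, opening the menu and its follow-up screens.
; On BeginPlay it shows the Menu widget, switches input to UI only and shows the mouse cursor.
; Separate events create and add the options and planet picker widgets to the viewport, and another quits the game.
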(event Custom|Show%20Options
  (bind _returnvalue (UserInterface|CreateWidget "/Game/ThirdPersonCPP/Blueprints/UI/Menu/MenuOptions.MenuOptions_C" (Game|GetPlayerController 0)))
  (UserInterface|Viewport|AddtoViewport _returnvalue 0))

(event Custom|Quit%20Game
  (Game|QuitGame (Game|GetPlayerController 0) "Quit"))

(event Custom|Show%20Menu
  (bind _returnvalue (UserInterface|CreateWidget "/Game/ThirdPersonCPP/Blueprints/UI/Menu/Menu.Menu_C" (Game|GetPlayerController 0)))
  (UserInterface|Viewport|AddtoViewport _returnvalue 0))

(event Custom|Pick%20a%20level
  (bind _returnvalue (UserInterface|CreateWidget "/Game/ThirdPersonCPP/Blueprints/UI/PlanetPickerWidget.PlanetPickerWidget_C"))
  (UserInterface|Viewport|AddtoViewport _returnvalue 0))

(event EventBeginPlay
  (CallFunction|ShowMenu)
  (Input|SetInputModeUIOnly 0 0 false)
  (Variables|/Script/Engine.PlayerController|SetbShowMouseCursor (Game|GetPlayerController 0) true))

(fn ConstructionScript)